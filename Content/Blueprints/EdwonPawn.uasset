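; EdwonPawn is a pawn that moves forward along its local X axis while thrust is toggled on.
; Each press of the Thrust input action flips a boolean, which Tick uses to gate a frame-rate-independent, non-swept offset scaled by Speed.
; Tick also prints the toggle state on screen for debugging, and the Right and Left sections are empty placeholders.
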(event `self.ReceiveBeginPlay`)

(event `self.ReceiveActorBeginOverlap`
  (params (OtherActor :type "Actor Object Reference")))

(event `self.ReceiveTick`
  (params (DeltaSeconds :type "Float (single-precision)"))
  (`KismetSystemLibrary.PrintString` (`KismetStringLibrary.Conv_BoolToString` (stale `InputAction|Thrust` _isa)) true false)
  (`self.K2_AddActorLocalOffset` (`KismetMathLibrary.MakeVector` (* (* (`KismetMathLibrary.SelectFloat` 1.0 0.0 (stale `InputAction|Thrust` _isa)) (`self.speed`)) (`GameplayStatics.GetWorldDeltaSeconds`)))))

(event `InputAction|Thrust`
  (:`Pressed`
    (bind _isa (`/Engine/EditorBlueprintResources/StandardMacros.FlipFlop`))))

(event `InputAction|Right`)

(event `InputAction|Left`)

(fn `UserConstructionScript`)
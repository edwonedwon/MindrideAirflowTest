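; EdwonPlayerController turns Thrust, Right and Left inputs into simple thrust-and-turn movement applied to its own actor.
; Input actions set booleans that Tick reads to build a damped forward velocity, moving the actor along local X without sweeping.
; Left and Right apply local roll rather than yaw, at a per-frame rate not scaled by delta time, with a debug print of that rate.
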(event `self.ReceiveBeginPlay`)

(event `self.ReceiveActorBeginOverlap`
  (params (OtherActor :type "Actor Object Reference")))

(event `self.ReceiveTick`
  (params (DeltaSeconds :type "Float (single-precision)"))
  (bind _rotationspeed (`self.rotationSpeed`))
  ;[1 1 1] THRUST
  (bind _output_get (set `self.velocity` (* (+ (* (* (`KismetMathLibrary.SelectFloat` 1.0 0.0 (`self.thrusting?`)) (`self.speed`)) (`GameplayStatics.GetWorldDeltaSeconds`)) (`self.velocity`)) (`self.damping`))))
  (`self.K2_AddActorLocalOffset` (`KismetMathLibrary.MakeVector` _output_get))
  ;[1 1 1] TURNING
  (bind _output_get_2 (set `self.rotationVelocity` (+ (`KismetMathLibrary.SelectFloat` _rotationspeed 0.0 (`self.right?`)) (`KismetMathLibrary.SelectFloat` (* _rotationspeed -1.0) 0.0 (`self.left?`)))))
  (`KismetSystemLibrary.PrintString` (`KismetStringLibrary.Conv_DoubleToString` _output_get_2))
  (`self.K2_AddActorLocalRotation` (`KismetMathLibrary.MakeRot` 0.0 0.0 _output_get_2)))

(event `InputAction|Thrust`
  ;[1 1 1] THRUST
  (:`Pressed`
    ;;[1 1 1] Set Thrusting Bool
    (set `self.thrusting?` true))
  (:`Released`
    (set `self.thrusting?` false)))

(event `InputAction|Right`
  ;[1 1 1] TURNING
  (:`Pressed`
    (set `self.right?` true))
  (:`Released`
    (set `self.right?` false)))

(event `InputAction|Left`
  ;[1 1 1] TURNING
  (:`Pressed`
    (set `self.left?` true))
  (:`Released`
    (set `self.left?` false)))

(fn `UserConstructionScript`)